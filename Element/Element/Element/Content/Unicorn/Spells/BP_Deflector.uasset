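; BP_Deflector is a forcefield shield spell that redirects non-team actors overlapping it along the shield's forward vector, passing along its team information.
; While the spell is active, Tick compares KinematicTracker velocity to a minimum activation speed.
; Start and end timers debounce the deflecting state, which toggles the mesh's visibility and query-only collision on mesh and box.
; Deactivating the spell immediately hides the shield and disables its collision.
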(event `self.ReceiveActorBeginOverlap`
  (params (OtherActor :type "Actor Object Reference"))
  ;[1 1 1] If deflecting, deflect actors in the direction the shield is facing
  (bind _returnvalue (`self.ImmuneToPrpjectiles`))
  (if _returnvalue
    (if (not (`TeamComponent.IsSameTeam` (`self.Team`) OtherActor))
      (message `/Game/Unicorn/Spells/BPI_Deflectable.Deflect` OtherActor (`self.GetActorForwardVector`) (`TeamComponent.Team` (`self.Team`)) (`TeamComponent.EnemyTeam` (`self.Team`))))))

(event `DeflectionStartTimerExpired`
  (set `self.bDeflecting` true)
  (set `self.bStartDeflectionTimerQueued` false)
  (`SceneComponent.SetVisibility` (`self.Mesh`) true false)
  (`PrimitiveComponent.SetCollisionEnabled` (`self.Mesh`) "QueryOnly")
  (`PrimitiveComponent.SetCollisionEnabled` (`self.Box`) "QueryOnly"))

(event `EndDeflectionTimerExpired`
  (set `self.bDeflecting` false)
  (set `self.bEndDeflectionTimerQueued` false)
  (`SceneComponent.SetVisibility` (`self.Mesh`) false false)
  (`PrimitiveComponent.SetCollisionEnabled` (`self.Mesh`) "NoCollision")
  (`PrimitiveComponent.SetCollisionEnabled` (`self.Box`) "NoCollision"))

(event `self.ReceiveTick`
  (params (DeltaSeconds :type "Float (single-precision)"))
  (if (`self.bSpellActive`)
    (if (>= (`KismetMathLibrary.VSize` (`/Game/Unicorn/Core/Engine/BP_KinematicVelocity_Component.GetKinematicVelocity` (`self.KinematicTracker`))) (`self.MinActivationVelocity`))
      (if (`self.bDeflecting`)
        (if (`self.bEndDeflectionTimerQueued`)
          (`KismetSystemLibrary.K2_ClearAndInvalidateTimerHandle` (`self.DeflectionEndTimer`))
          (set `self.bEndDeflectionTimerQueued` false))
        (elif (not (`self.bStartDeflectionTimerQueued`))
          (bind _returnvalue (`KismetSystemLibrary.K2_SetTimerDelegate` (`|CreateDelegate` :!event `DeflectionStartTimerExpired`) (`self.ActivationToggleTime`)))
          (set `self.DeflectionStartTimer` _returnvalue)
          (set `self.bStartDeflectionTimerQueued` true)))
      (elif (`self.bDeflecting`)
        (if (not (`self.bEndDeflectionTimerQueued`))
          (bind _returnvalue_2 (`KismetSystemLibrary.K2_SetTimerDelegate` (`|CreateDelegate` :!event `EndDeflectionTimerExpired`) (`self.DeactivationToggleTime`)))
          (set `self.DeflectionEndTimer` _returnvalue_2)
          (set `self.bEndDeflectionTimerQueued` true))
        (elif (`self.bStartDeflectionTimerQueued`)
          (`KismetSystemLibrary.K2_ClearAndInvalidateTimerHandle` (`self.DeflectionStartTimer`))
          (set `self.bStartDeflectionTimerQueued` false))))))

(event `self.ActivateSpell`
  (`parent.ActivateSpell`))

(event `self.DeactivateSpell`
  (`parent.DeactivateSpell`)
  (set `self.bDeflecting` false)
  (`SceneComponent.SetVisibility` (`self.Mesh`) false false)
  (`PrimitiveComponent.SetCollisionEnabled` (`self.Mesh`) "NoCollision")
  (`PrimitiveComponent.SetCollisionEnabled` (`self.Box`) "NoCollision"))

(fn `ImmuneToPrpjectiles`
  (returns (ReturnValue :type Boolean))
  (if (`self.bSpellActive`)
    ;[1 1 1] Check whether we are moving fast enough to deflect projectiles
    (return (`self.bDeflecting`))
    (else
      (return false))))

(fn `UserConstructionScript`
  ;[1 1 1] Get a reference to our forcefield mat so we can adjust it later
  (bind _returnvalue (`KismetMaterialLibrary.CreateDynamicMaterialInstance` "/Game/Unicorn/Spells/M_ForceField.M_ForceField"))
  (bind _output_get (set `self.ForceFieldMat` _returnvalue))
  (`PrimitiveComponent.SetMaterial` (`self.Mesh`) 0 _output_get))