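; BP_FireSwipe is a fire spell projectile that stuns and knocks back enemies it hits.
; A one-shot timer enables rotation after a delay.
; Tick then turns the actor toward a target rotation at constant speed while no valid TargetActor exists, reapplying local-space velocity to curve its path.
; HitEnemy calls the parent, plays an attached blast sound, and applies stun and knockback only when the parent returns false.
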(event `self.ReceiveBeginPlay`
  (`parent.ReceiveBeginPlay`)
  (`KismetSystemLibrary.K2_SetTimerDelegate` (`|CreateDelegate` :!event `RotationDelayTimerExpired`) (`self.RotationDelay`)))

(event `RotationDelayTimerExpired`
  (set `self.bRotating` true))

(event `self.ReceiveTick`
  (params (DeltaSeconds :type "Float (single-precision)"))
  (`parent.ReceiveTick` DeltaSeconds)
  (if (`self.bRotating`)
    (`/Engine/EditorBlueprintResources/StandardMacros.IsValid` (`self.TargetActor`)
      (:`Is Not Valid`
        (`self.K2_SetActorRotation` (`KismetMathLibrary.RInterpTo_Constant` (`self.K2_GetActorRotation`) (`self.TargetRotation`) (`GameplayStatics.GetWorldDeltaSeconds`) (`self.RotationSpeed`)))
        (`ProjectileMovementComponent.SetVelocityInLocalSpace` (`self.ProjectileMovement`) (`self.ProjectileVelocity`))))))

(fn `HitEnemy`
  (params (Enemy :type "Actor Object Reference"))
  (returns (Died :type Boolean))
  (bind _died (`parent.HitEnemy` Enemy))
  (`GameplayStatics.SpawnSoundAttached` "/Game/ProSoundCollection_v1_3/Magic_Spells/Cues/fireball_blast_projectile_spell_06_Cue.fireball_blast_projectile_spell_06_Cue" (`self.RootComponent`) "None" (0.0 0.0 0.0) (struct) "KeepRelativeOffset" false 1.0 1.0 0.0 "/Game/ATT_Spell.ATT_Spell" "/Game/CON_Spell.CON_Spell")
  (if (not _died)
    (message `/Game/Unicorn/Core/Engine/BPI_Stunnable.BeStunned` Enemy (`self.StunPower`))
    (message `/Game/Unicorn/Core/Engine/BPI_Knockback.Knockback` Enemy (`self.K2_GetActorLocation`) (`self.KnockbackForce`))
    (return _died)))

(fn `UserConstructionScript`
  (`parent.UserConstructionScript`))