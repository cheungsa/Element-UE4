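; Base-style projectile spell that damages non-allied actors on overlap, respecting projectile immunity and clash power.
; On spawn it can snap aim, within an angle limit, toward a given target or the best-aligned visible enemy, then optionally homes.
; A timeline scales the mesh up, starts the lifetime timer, and reverses on deactivation to shrink and destroy it.
; Deflection switches its team to the deflector's without changing direction.
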(event `self.ReceiveBeginPlay`
  (bind _aimassistdesireddirection (`self.AimAssistDesiredDirection`))
  (`parent.ReceiveBeginPlay`)
  ;[1 1 1] Hit all actors we are already overlapping
  (`self.ActivateSpell`)
  (for _array_element (`self.GetOverlappingActors` null)
    (`self.HitActor` _array_element))
  ;[1 1 1] Initialize projectile velocity
  (`ProjectileMovementComponent.SetVelocityInLocalSpace` (`self.ProjectileMovement`) (`self.ProjectileVelocity`))
  ;[1 1 1] Handle aim assist if enabled
  (`/Engine/EditorBlueprintResources/StandardMacros.IsValid` (`self.TargetActor`)
    (:`Is Valid`
      ;[1 1 1] If we have been provided with a target actor, try to rotate towards it
      (`self.K2_SetActorRotation` (`KismetMathLibrary.RInterpTo_Constant` (`self.K2_GetActorRotation`) (`KismetMathLibrary.FindLookAtRotation` (`self.K2_GetActorLocation`) (`UnicornFunctionLibrary.GetAimLocationOnActor` (`self.TargetActor`))) 1.0 (`self.AimAssistMaxAssistAngle`))))
    (:`Is Not Valid`
      (`/Engine/EditorBlueprintResources/StandardMacros.IsValid` self
        (:`Is Valid`
          (if (`self.bAimAssist`)
            (bind (_success _returnvalue _besttargetaimlocation) (`self.GetBestTarget` (select `bool` (== _aimassistdesireddirection (0.0 0.0 0.0)) :`false` _aimassistdesireddirection :`true` (`SceneComponent.GetForwardVector` (`self.DefaultSceneRoot`))) (`self.AimAssistAngleTolerance`)))
            (if _success
              (set `self.TargetActor` _returnvalue)
              (`self.K2_SetActorRotation` (`KismetMathLibrary.RInterpTo_Constant` (`self.K2_GetActorRotation`) (`KismetMathLibrary.FindLookAtRotation` (`self.K2_GetActorLocation`) _besttargetaimlocation) 1.0 (`self.AimAssistMaxAssistAngle`))))))))))

(event `self.ReceiveActorBeginOverlap`
  (params (OtherActor :type "Actor Object Reference"))
  (`self.HitActor` OtherActor))

(event `self.ReceiveTick`
  (params (DeltaSeconds :type "Float (single-precision)"))
  (`parent.ReceiveTick` DeltaSeconds)
  (`|ExecutionSequence`
    (:`then_0`
      ;[1 1 1] Manage growth state
      (switch `/Game/Unicorn/Core/Engine/EGrowthState` (`self.CurrGrowthState`)
        (:`NewEnumerator1`
          (bind (_direction _projectilescale) (`Timeline|GrowthTimeline` :!label _label)
            (:`Update`
              (`SceneComponent.SetRelativeScale3D` (`self.Mesh`) (`KismetMathLibrary.VLerp` (`self.ProjectileShrinkSize`) (`self.ProjectileFullSize`) _projectilescale)))
            (:`Finished`
              (switch `ETimelineDirection` _direction
                (:`Forward`
                  (set `self.CurrGrowthState` "NewEnumerator3")
                  (`KismetSystemLibrary.K2_SetTimerDelegate` (delegate `LifetimeTimerExpired`) (`self.Lifetime`)))
                (:`Backward`
                  (`self.K2_DestroyActor` self))))))
        (:`NewEnumerator2`
          (goto _label :!via `Reverse`))))
    (:`then_1`
      ;[1 1 1] If homing was enabled, continue to turn towards the target
      (if (and (`self.bHoming`) (`KismetSystemLibrary.IsValid` (`self.TargetActor`)))
        (`self.K2_SetActorRotation` (`KismetMathLibrary.RInterpTo` (`self.K2_GetActorRotation`) (`KismetMathLibrary.FindLookAtRotation` (`self.K2_GetActorLocation`) (`UnicornFunctionLibrary.GetAimLocationOnActor` (`self.TargetActor`))) (`GameplayStatics.GetWorldDeltaSeconds`) (`self.HomingRotationSpeed`)))
        (`ProjectileMovementComponent.SetVelocityInLocalSpace` (`self.ProjectileMovement`) (`self.ProjectileVelocity`))))))

(event `LifetimeTimerExpired`
  (`self.SafeDeactivateSpell`))

(event `self.DeactivateSpell`
  (`parent.DeactivateSpell`)
  (set `self.CurrGrowthState` "NewEnumerator2"))

(fn `Deflect`
  (params (DeflectorDirection :type "Vector Structure") (DeflectorTeam :type "ETeam Enum" :default "TE_Player") (DeflectorEnemyTeam :type "ETeam Enum" :default "TE_Player"))
  (returns (Success :type Boolean))
  (bind _output_get (set `self.SpellTeam` DeflectorTeam))
  (set `TeamComponent.Team` _output_get (`self.Team`))
  (bind _output_get_2 (set `TeamComponent.EnemyTeam` DeflectorEnemyTeam (`self.Team`)))
  (set `self.SpellEnemyTeam` _output_get_2)
  (return true))

(fn `GetBestTarget`
  (params (`Desired Direction` :type "Vector Structure") (AngleTolerance :type "Float (double-precision)"))
  (returns (Success :type Boolean) (ReturnValue :type "Actor Object Reference") (BestTargetAimLocation :type "Vector Structure"))
  (locals (CurrTarget :type "Actor Object Reference") (BestTarget :type "Actor Object Reference") (DirectionToCurrTarget :type "Vector Structure") (CurrTargetScore :type "Float (double-precision)") (BestTargetScore :type "Float (double-precision)" :default -100.0) (FoundTarget :type Boolean) (CurrAimLocation :type "Vector Structure") (BestAimLocation :type "Vector Structure"))
  (bind _returnvalue (`self.K2_GetActorLocation`))
  ;[1 1 1] Get all actors within range
  (`|ExecutionSequence`
    (:`then_0`
      (bind (_outhits _returnvalue_2) (`KismetSystemLibrary.SphereTraceMulti` _returnvalue (+ _returnvalue 0.1) (* (`self.Lifetime`) (`KismetMathLibrary.VSize` (`self.ProjectileVelocity`))) "TraceTypeQuery2"))
      ;[1 1 1] Filter by enemy actors and valid targets
      (if _returnvalue_2
        (for _array_element _outhits
          (bind _output_get (set `local.CurrTarget` (`.HitActor` (`GameplayStatics.BreakHitResult` _array_element))))
          (`/Engine/EditorBlueprintResources/StandardMacros.IsValid` _output_get
            (:`Is Valid`
              (if (`TeamComponent.IsEnemyTeam` (`self.Team`) _output_get)
                ;[1 1 1] Score and filter targets by angle
                (bind _output_get_2 (set `local.CurrAimLocation` (`UnicornFunctionLibrary.GetAimLocationOnActor` (`local.CurrTarget`) (`self.VRAimLocationHeightMultiplier`))))
                (bind _output_get_3 (set `local.DirectionToCurrTarget` (`KismetMathLibrary.Normal` (- _output_get_2 (`self.K2_GetActorLocation`)))))
                (bind _output_get_4 (set `local.CurrTargetScore` (`KismetMathLibrary.Dot_VectorVector` _output_get_3 (`local.Desired Direction`))))
                (bind _outhit (`KismetSystemLibrary.LineTraceSingle` (`self.K2_GetActorLocation`) (`local.CurrAimLocation`) "TraceTypeQuery2"))
                (if (== (`.HitActor` (`GameplayStatics.BreakHitResult` _outhit)) (`local.CurrTarget`))
                  (if (and (>= _output_get_4 (`KismetMathLibrary.DegCos` (`local.AngleTolerance`))) (> (`local.CurrTargetScore`) (`local.BestTargetScore`)))
                    (set `local.BestTarget` (`local.CurrTarget`))
                    (set `local.BestTargetScore` (`local.CurrTargetScore`))
                    (set `local.BestAimLocation` (`local.CurrAimLocation`))
                    (set `local.FoundTarget` true)))))))))
    (:`then_1`
      (return (`local.FoundTarget`) (`local.BestTarget`) (`local.BestAimLocation`)))))

(fn `HitActor`
  (params (HitActor :type "Actor Object Reference"))
  ;[1 1 1] Check if we are active
  (`|ExecutionSequence`
    (:`then_0`
      (if (`self.bSpellActive`)
        ;[1 1 1] Check in the overlapped actor is the same team (we don't want friendly fire)
        (if (not (`TeamComponent.IsSameTeam` (`self.Team`) (`local.HitActor`)))
          ;[1 1 1] Check if the actor is deflecting or has a higher clash rating
          (bind _returnvalue (message `/Game/Unicorn/Spells/BPI_ProjectileImmunity.ImmuneToPrpjectiles` (`local.HitActor`)))
          (if (not _returnvalue)
            (bind _returnvalue_2 (message `/Game/Unicorn/Core/Engine/BPI_Clashasble.ShouldWinClash` (`local.HitActor`) (`self.ClashPower`)))
            (if (not _returnvalue_2)
              (`self.HitEnemy` (`local.HitActor`)))
            (`self.DeactivateSpell`)
            (return)))))
    (:`then_1`
      (return))))

(fn `HitEnemy`
  (params (Enemy :type "Actor Object Reference"))
  (returns (Died :type Boolean))
  ;[1 1 1] If all the conditions are cleared, damage the other actor and destroy this fireball
  (set `self.bHoming` false)
  (bind _bdied (message `HealthInterface.LoseHealth` (`local.Enemy`) (`self.DamageAmount`)))
  (return _bdied))

(fn `ShouldWinClash`
  (params (ClashPower :type "/Game/Unicorn/Core/Engine/EPowerLevel Enum" :default "NewEnumerator0"))
  (returns (ReturnValue :type Boolean))
  (return (< ClashPower (`self.ClashPower`))))

(fn `UserConstructionScript`
  (`parent.UserConstructionScript`))