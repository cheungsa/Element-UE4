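; Fire shield spell actor that damages non-team actors on entry and overlapping non-team pawns every second they remain, and reports itself immune to projectiles.
; On spawn it plays a sound and scales WallAnchor up through a timeline driven from Tick, then starts a lifetime timer.
; It deactivates and destroys itself when that timer expires or the owner's VR location moves horizontally beyond its radius.
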(event `self.ReceiveBeginPlay`
  (`self.ActivateSpell`)
  (set `self.CurrShieldGrowthState` "NewEnumerator1")
  (`GameplayStatics.SpawnSoundAttached` "/Game/ProSoundCollection_v1_3/Magic_Spells/Cues/casting_charge_whoosh_buildup4_Cue.casting_charge_whoosh_buildup4_Cue" (`self.RootComponent`) "None" (0.0 0.0 0.0) (struct) "KeepRelativeOffset" false 1.0 1.0 0.0 "/Game/ATT_Spell.ATT_Spell" "/Game/CON_Spell.CON_Spell"))

(event `OnLifetimeTimerExpired`
  ;[1 1 1] Set a deactivation timer as appropriate
  (`self.DeactivateSpell`))

(event `self.ReceiveTick`
  (params (DeltaSeconds :type "Float (single-precision)"))
  (`parent.ReceiveTick` DeltaSeconds)
  (`|ExecutionSequence`
    (:`then_0`
      ;[1 1 1] Handle growing and shrinking the shield when spawning and dying
      (switch `/Game/Unicorn/Core/Engine/EGrowthState` (`self.CurrShieldGrowthState`)
        (:`NewEnumerator1`
          (bind (_direction _growth) (`Timeline|GrowthTimeline`)
            (:`Update`
              (`SceneComponent.SetRelativeScale3D` (`self.WallAnchor`) (`KismetMathLibrary.VLerp` (`self.ShieldMinSize`) (`self.ShieldMaxSize`) _growth)))
            (:`Finished`
              (set `self.CurrShieldGrowthState` "NewEnumerator3")
              ;[1 1 1] Set a deactivation timer as appropriate
              (bind _returnvalue (`KismetSystemLibrary.K2_SetTimerDelegate` (delegate `OnLifetimeTimerExpired`) (`self.ShieldLifetime`)))
              (set `self.ShieldLifetimeTmer` _returnvalue))))))
    (:`then_1`
      (for _array_element (`self.GetOverlappingActors` "/Script/Engine.Pawn")
        (if (not (`TeamComponent.IsSameTeam` (`self.Team`) _array_element))
          (message `HealthInterface.LoseHealth` _array_element (* (`self.DamagePerSecond`) (`GameplayStatics.GetWorldDeltaSeconds`))))))
    (:`then_2`
      ;[1 1 1] Deactivate the spell when we get too far away
      (if (`self.bSpellActive`)
        (if (> (`KismetMathLibrary.VSize` (`/Game/Unicorn/Core/Engine/BPFL_UnicornLibrary.FlattenZ` (- (`VRBaseCharacter.GetVRLocation` (`self.ShieldOwner`)) (`self.K2_GetActorLocation`)))) (`self.Radius`))
          (`KismetSystemLibrary.K2_ClearAndInvalidateTimerHandle` (`self.ShieldLifetimeTmer`))
          (`self.DeactivateSpell`))))))

(event `self.ReceiveActorBeginOverlap`
  (params (OtherActor :type "Actor Object Reference"))
  (if (not (`TeamComponent.IsSameTeam` (`self.Team`) OtherActor))
    (message `HealthInterface.LoseHealth` OtherActor (`self.EntryDamage`))))

(event `self.DeactivateSpell`
  (`parent.DeactivateSpell`)
  (`self.K2_DestroyActor`))

(fn `ImmuneToPrpjectiles`
  (returns (ReturnValue :type Boolean))
  (return true))

(fn `UserConstructionScript`)