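; BP_ForceBall is a force ball spell Blueprint that stuns and knocks back the enemies it hits.
; It overrides HitEnemy, calling the parent first and playing an attached impact sound on every call.
; Only when the parent returns false does it message the enemy to be stunned and knocked back from the ball's location.
; All other events and construction defer to the parent class.
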(event `self.ReceiveBeginPlay`
  (`parent.ReceiveBeginPlay`))

(fn `HitEnemy`
  (params (Enemy :type "Actor Object Reference"))
  (returns (Died :type Boolean))
  (bind _died (`parent.HitEnemy` Enemy))
  (`GameplayStatics.SpawnSoundAttached` "/Game/ProSoundCollection_v1_3/Magic_Spells/Cues/fireball_blast_projectile_spell_06_Cue.fireball_blast_projectile_spell_06_Cue" (`self.RootComponent`) "None" (0.0 0.0 0.0) (struct) "KeepRelativeOffset" false 1.0 1.0 0.0 "/Game/ATT_Spell.ATT_Spell" "/Game/CON_Spell.CON_Spell")
  (if (not _died)
    (message `/Game/Unicorn/Core/Engine/BPI_Stunnable.BeStunned` Enemy (`self.StunPower`))
    (message `/Game/Unicorn/Core/Engine/BPI_Knockback.Knockback` Enemy (`self.K2_GetActorLocation`) (`self.KnockbackForce`))
    (return _died)))

(fn `UserConstructionScript`
  (`parent.UserConstructionScript`))