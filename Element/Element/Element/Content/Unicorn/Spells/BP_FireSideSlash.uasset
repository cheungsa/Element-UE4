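; Fire side slash spell projectile that turns as it flies, following a curved path.
; On BeginPlay it caches its speed and initial forward direction.
; Each Tick it rotates around its up vector by YawChange and RotationSpeed, then resets ProjectileMovement's local velocity.
; That velocity blends current forward with launch direction, weighted by MinInitialForwardVelocity, and is normalized to keep speed constant while retaining a bias along the original heading.
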(event `self.ReceiveBeginPlay`
  (`parent.ReceiveBeginPlay`)
  (set `self.VelocityLength` (`KismetMathLibrary.VSize` (`self.ProjectileVelocity`)))
  (set `self.InitialForward` (`self.GetActorForwardVector`)))

(event `self.ReceiveTick`
  (params (DeltaSeconds :type "Float (single-precision)"))
  (`parent.ReceiveTick` DeltaSeconds)
  (`self.K2_SetActorRotation` (`KismetMathLibrary.ComposeRotators` (`self.K2_GetActorRotation`) (`KismetMathLibrary.RotatorFromAxisAndAngle` (`self.GetActorUpVector`) (* (`GameplayStatics.GetWorldDeltaSeconds`) (`self.YawChange`) (`self.RotationSpeed`)))))
  (`ProjectileMovementComponent.SetVelocityInLocalSpace` (`self.ProjectileMovement`) (* (`KismetMathLibrary.Normal` (+ (`KismetMathLibrary.InverseTransformDirection` (`self.GetTransform`) (* (`self.InitialForward`) (`self.MinInitialForwardVelocity`))) (* (1.0 0.0 0.0) (- 1.0 (`self.MinInitialForwardVelocity`))))) (`self.VelocityLength`))))

(fn `UserConstructionScript`
  (`parent.UserConstructionScript`))