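; BP_IceSpike is an ice projectile spell that builds on a parent spell class for overlap, hit and deflection logic.
; It adds attached, attenuated sounds for launch, enemy hit and deflection.
; Deflection flips the actor to face backward and reapplies its velocity in local space through the projectile movement component.
; Deactivation zeroes the stored projectile velocity, and construction clears the lifespan.
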(event `self.ReceiveBeginPlay`
  (`parent.ReceiveBeginPlay`)
  (`GameplayStatics.SpawnSoundAttached` "/Game/ProSoundCollection_v1_3/Magic_Spells/Cues/ice_blast_projectile_spell_04_Cue.ice_blast_projectile_spell_04_Cue" (`self.RootComponent`) "None" (0.0 0.0 0.0) (struct) "KeepRelativeOffset" false 1.0 1.0 0.0 "/Game/ATT_Spell.ATT_Spell" "/Game/CON_Spell.CON_Spell"))

(event `self.ReceiveActorBeginOverlap`
  (params (OtherActor :type "Actor Object Reference"))
  (`parent.ReceiveActorBeginOverlap` OtherActor))

(event `self.ReceiveTick`
  (params (DeltaSeconds :type "Float (single-precision)"))
  (`parent.ReceiveTick` DeltaSeconds))

(event `/Game/Unicorn/Spells/BP_Spell_Base.DeactivateSpell`
  (set `self.ProjectileVelocity` (0.0 0.0 0.0))
  (`parent.DeactivateSpell`))

(fn `Deflect`
  (params (DeflectorDirection :type "Vector Structure") (DeflectorTeam :type "ETeam Enum" :default "TE_Player") (DeflectorEnemyTeam :type "ETeam Enum" :default "TE_Player"))
  (returns (Success :type Boolean))
  (`parent.Deflect` DeflectorDirection DeflectorTeam DeflectorEnemyTeam)
  (`self.K2_SetActorRotation` (`KismetMathLibrary.MakeRotFromX` (* (`self.GetActorForwardVector`) -1.0)))
  (`ProjectileMovementComponent.SetVelocityInLocalSpace` (`self.ProjectileMovement`) (`self.ProjectileVelocity`))
  (`GameplayStatics.SpawnSoundAttached` "/Game/ProSoundCollection_v1_3/Magic_Spells/Cues/fireball_projectile_deflect_02_Cue.fireball_projectile_deflect_02_Cue" (`self.RootComponent`) "None" (0.0 0.0 0.0) (struct) "KeepRelativeOffset" false 1.0 1.0 0.0 "/Game/ATT_Spell.ATT_Spell" "/Game/CON_Spell.CON_Spell")
  (return true))

(fn `HitEnemy`
  (params (Enemy :type "Actor Object Reference"))
  (returns (Died :type Boolean))
  (`GameplayStatics.SpawnSoundAttached` "/Game/ProSoundCollection_v1_3/Magic_Spells/Cues/ice_spell_freeze_frost_03_Cue.ice_spell_freeze_frost_03_Cue" (`self.RootComponent`) "None" (0.0 0.0 0.0) (struct) "KeepRelativeOffset" false 1.0 1.0 0.0 "/Game/ATT_Spell.ATT_Spell" "/Game/CON_Spell.CON_Spell")
  (bind _died (`parent.HitEnemy` Enemy))
  (return _died))

(fn `UserConstructionScript`
  (`parent.UserConstructionScript`)
  (`self.SetLifeSpan` 0.0))