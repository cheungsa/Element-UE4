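; Fireball spell projectile, a child of a spell base class, that stuns and knocks back enemies it hits.
; It plays an attached launch sound on BeginPlay.
; Its HitEnemy override spawns an explosion effect and sound, sends stun and knockback messages to the enemy, then calls the parent.
; Deactivation calls the parent, then disables named emitters on the fire trail and ball.
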(event `self.ReceiveBeginPlay`
  (`parent.ReceiveBeginPlay`)
  (`GameplayStatics.SpawnSoundAttached` "/Game/ProSoundCollection_v1_3/Magic_Spells/Cues/fireball_blast_projectile_spell_01_Cue.fireball_blast_projectile_spell_01_Cue" (`self.DefaultSceneRoot`) "None" (0.0 0.0 0.0) (struct) "KeepRelativeOffset" false 1.0 1.0 0.0 "/Game/ATT_Spell.ATT_Spell" "/Game/CON_Spell.CON_Spell"))

(event `self.DeactivateSpell`
  (`parent.DeactivateSpell`)
  (`ParticleSystemComponent.SetEmitterEnable` (`self.FireTrail`) "FireBase3" false)
  (`ParticleSystemComponent.SetEmitterEnable` (`self.FireTrail`) "SmokePuff2" false)
  (`ParticleSystemComponent.SetEmitterEnable` (`self.FireTrail`) "SmokePuff3" false)
  (`ParticleSystemComponent.SetEmitterEnable` (`self.FireBall`) "FireBall5" false))

(fn `HitEnemy`
  (params (Enemy :type "Actor Object Reference"))
  (returns (Died :type Boolean))
  (`GameplayStatics.SpawnEmitterAtLocation` "/Game/Unicorn/ParticleAssets/P_FireballExplosion.P_FireballExplosion" (`self.K2_GetActorLocation`) (struct) (0.5 0.5 0.5))
  (`GameplayStatics.SpawnSoundAttached` "/Game/ProSoundCollection_v1_3/Magic_Spells/Cues/fireball_blast_projectile_spell_06_Cue.fireball_blast_projectile_spell_06_Cue" (`self.RootComponent`) "None" (0.0 0.0 0.0) (struct) "KeepRelativeOffset" false 1.0 1.0 0.0 "/Game/ATT_Spell.ATT_Spell" "/Game/CON_Spell.CON_Spell")
  (message `/Game/Unicorn/Core/Engine/BPI_Stunnable.BeStunned` (`local.Enemy`) (`self.StunPower`))
  (message `/Game/Unicorn/Core/Engine/BPI_Knockback.Knockback` (`local.Enemy`) (`self.K2_GetActorLocation`) (`self.KnockbackForce`))
  (bind _died (`parent.HitEnemy` (`local.Enemy`)))
  (return _died))

(fn `UserConstructionScript`
  (`parent.UserConstructionScript`))