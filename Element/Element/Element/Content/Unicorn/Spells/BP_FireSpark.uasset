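; BP_FireSpark is a fire spark spell Blueprint that can stun the enemies it hits.
; It overrides HitEnemy, running the parent's hit logic first and sending the enemy a BeStunned interface message with StunPower only when that logic returns false.
; The event graph holds only disabled default events and the construction script just calls the parent, so all other behavior is inherited.
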(fn `HitEnemy`
  (params (Enemy :type "Actor Object Reference"))
  (returns (Died :type Boolean))
  (bind _died (`parent.HitEnemy` Enemy))
  (if (not _died)
    (message `/Game/Unicorn/Core/Engine/BPI_Stunnable.BeStunned` (`local.Enemy`) (`self.StunPower`))
    (return _died)))

(fn `UserConstructionScript`
  (`parent.UserConstructionScript`))