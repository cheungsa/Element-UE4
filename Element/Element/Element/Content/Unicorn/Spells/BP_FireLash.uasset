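; Fire lash spell that throws fire sparks while the spell is active and swept fast enough sideways or vertically.
; Each tick, KinematicTracker velocity along its up and right axes gates an activation timer, which enables fire emitters, audio and spawning.
; Slowing down stops the fire, while sharp direction reversals restart the timer.
; BP_TurningFireSpark actors spawn at fixed spacing along the travelled path, avoiding frame-rate gaps, inheriting damage and teams.
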(event `self.ReceiveBeginPlay`
  (`parent.ReceiveBeginPlay`)
  (`self.SetEmittersActive` false)
  (`SceneComponent.SetWorldScale3D` (`self.ParticleSystem`) (1.0 1.0 1.0))
  (`AudioComponent.Stop` (`self.Audio`)))

(event `self.DeactivateSpell`
  (`parent.DeactivateSpell`)
  (set `self.bSpawningFire` false)
  (set `self.bCurrHasActivationVelocity` false)
  (set `self.bLastHadActivationVelocity` false)
  (`self.SetEmittersActive` false)
  (`AudioComponent.Stop` (`self.Audio`)))

(event `LashActivationTimerFinished`
  (set `self.bSpawningFire` true)
  (set `self.LastSpawnedPosition` (`self.K2_GetActorLocation`))
  (`self.SetEmittersActive` true)
  (`AudioComponent.Play` (`self.Audio`) 0.0))

(event `self.ReceiveTick`
  (params (DeltaSeconds :type "Float (single-precision)"))
  (bind _kinematictracker (`self.KinematicTracker`))
  (bind _kinematictracker_2 (`self.KinematicTracker`))
  (bind _kinematictracker_3 (`self.KinematicTracker`))
  (bind _returnvalue (- (`self.K2_GetActorLocation`) (`self.LastSpawnedPosition`)))
  (if (`self.bSpellActive`)
    (`|ExecutionSequence`
      (:`then_0`
        (`|ExecutionSequence`
          (:`then_0`
            (bind _returnvalue_2 (`/Game/Unicorn/Core/Engine/BP_KinematicVelocity_Component.GetVelocityInDirection` _kinematictracker_2 (`SceneComponent.GetUpVector` _kinematictracker_2)))
            (bind _returnvalue_3 (`/Game/Unicorn/Core/Engine/BP_KinematicVelocity_Component.GetVelocityInDirection` _kinematictracker (`SceneComponent.GetRightVector` _kinematictracker)))
            (set `self.bCurrHasActivationVelocity` (>= (+ (`KismetMathLibrary.Abs` _returnvalue_3) (`KismetMathLibrary.Abs` _returnvalue_2)) (`self.MinActivationVelocity`))))
          (:`then_1`
            (if (`self.bCurrHasActivationVelocity`)
              (if (`self.bLastHadActivationVelocity`)
                (if (not (<= (`/Game/Unicorn/Core/Engine/BPFL_UnicornLibrary.GetAngleBetweenVectors` (`/Game/Unicorn/Core/Engine/BP_KinematicVelocity_Component.GetKinematicVelocity` _kinematictracker_3) (`/Game/Unicorn/Core/Engine/BP_KinematicVelocity_Component.GetLastKinematicVelocity` _kinematictracker_3)) (`self.LashReverseAngleTolerance`)))
                  (`KismetSystemLibrary.K2_ClearAndInvalidateTimerHandle` (`self.ActivationTimer`))
                  (set `self.bSpawningFire` false)
                  (`self.SetEmittersActive` false)
                  (`AudioComponent.Stop` (`self.Audio`))
                  (bind _returnvalue_4 (`KismetSystemLibrary.K2_SetTimerDelegate` (`|CreateDelegate` :!event `LashActivationTimerFinished`) (`self.MinLashActivationTime`) :!label _label))
                  (set `self.ActivationTimer` _returnvalue_4))
                (else
                  (goto _label)))
              (elif (`self.bLastHadActivationVelocity`)
                (`KismetSystemLibrary.K2_ClearAndInvalidateTimerHandle` (`self.ActivationTimer`))
                (set `self.bSpawningFire` false)
                (`self.SetEmittersActive` false)
                (`AudioComponent.Stop` (`self.Audio`)))))
          (:`then_2`
            (set `self.bLastHadActivationVelocity` (`self.bCurrHasActivationVelocity`)))))
      (:`then_1`
        (if (`self.bSpawningFire`)
          (set `self.CurrentJumps` 1)
          (set `self.FireDirectionNormalized` (`KismetMathLibrary.Normal` _returnvalue))
          (set `self.CurrFireSpawningDistance` (`KismetMathLibrary.VSize` _returnvalue))
          (while (<= (* (`self.CurrentJumps`) (`self.DistanceBetweenSpawnedFire`)) (`self.CurrFireSpawningDistance`))
            (bind _output_get (set `self.LastSpawnedPosition` (+ (`self.LastSpawnedPosition`) (* (`self.FireDirectionNormalized`) (`self.DistanceBetweenSpawnedFire`)))))
            (`|SpawnActorFromClass` "/Game/Unicorn/Spells/BP_TurningFireSpark.BP_TurningFireSpark_C" (`KismetMathLibrary.MakeTransform` _output_get (`KismetMathLibrary.MakeRotFromXY` (`SceneComponent.GetForwardVector` (`self.KinematicTracker`)) (`self.FireDirectionNormalized`))) "Undefined" "OverrideRootScale" null 0.5 30.0 (`self.DamageAmount`) (1000.0 0.0 0.0) 0.5 (0.5 1.0 0.1) false 50.0 (0.0 0.0 0.0) 25.0 null false 5.0 (`self.SpellTeam`) (`self.SpellEnemyTeam`) null)
            (`/Engine/EditorBlueprintResources/StandardMacros.IncrementInt` (`self.CurrentJumps`))))))))

(fn `SetEmittersActive`
  (params (NewActive :type Boolean))
  (`ParticleSystemComponent.SetEmitterEnable` (`self.ParticleSystem`) "FireField1" (`local.NewActive`))
  (`ParticleSystemComponent.SetEmitterEnable` (`self.ParticleSystem`) "FireField2" (`local.NewActive`))
  (return))

(fn `UserConstructionScript`
  (`parent.UserConstructionScript`))