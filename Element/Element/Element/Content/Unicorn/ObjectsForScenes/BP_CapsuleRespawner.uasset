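; BP_CapsuleRespawner is a scene actor that keeps two referenced capsule AI characters alive by respawning them when they are gone.
; BeginPlay records each capsule's starting location as its spawn point.
; Tick checks both references; when one is invalid, it waits a respawn delay, spawns that slot's class and behavior tree there, and stores the new reference.
; Per-slot flags block duplicate spawns during the delay.
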(event `self.ReceiveBeginPlay`
  (`|ExecutionSequence`
    (:`then_0`
      (set `self.Capsule01SpawnPoint` (`self.K2_GetActorLocation` (`self.Capsule01`))))
    (:`then_1`
      (set `self.Capsule02SpawnPoint` (`self.K2_GetActorLocation` (`self.Capsule02`))))))

(event `self.ReceiveTick`
  (params (DeltaSeconds :type "Float (single-precision)"))
  (`|ExecutionSequence`
    (:`then_0`
      (`/Engine/EditorBlueprintResources/StandardMacros.IsValid` (`self.Capsule01`)
        (:`Is Not Valid`
          (if (not (`self.SpawningCapsule01`))
            (set `self.SpawningCapsule01` true)
            (`KismetSystemLibrary.Delay` (`self.CapsuleRespawnTime`))
            (bind _returnvalue (`AIBlueprintHelperLibrary.SpawnAIFromClass` (`self.Capsule01Class`) (`self.Capsule01BT`) (`self.Capsule01SpawnPoint`)))
            (bind _asbp_capsule_character (cast `/Game/Unicorn/Characters/UnicornCharacter/BP_CapsuleCharacter` _returnvalue))
            (set `self.Capsule01` _asbp_capsule_character)
            (set `self.SpawningCapsule01` false)))))
    (:`then_1`
      (`/Engine/EditorBlueprintResources/StandardMacros.IsValid` (`self.Capsule02`)
        (:`Is Not Valid`
          (if (not (`self.SpawningCapsule02`))
            (set `self.SpawningCapsule02` true)
            (`KismetSystemLibrary.Delay` (`self.CapsuleRespawnTime`))
            (bind _returnvalue_2 (`AIBlueprintHelperLibrary.SpawnAIFromClass` (`self.Capsule02Class`) (`self.Capsule02BT`) (`self.Capsule02SpawnPoint`)))
            (bind _asbp_capsule_character_2 (cast `/Game/Unicorn/Characters/UnicornCharacter/BP_CapsuleCharacter` _returnvalue_2))
            (set `self.Capsule02` _asbp_capsule_character_2)
            (set `self.SpawningCapsule02` false)))))))

(fn `UserConstructionScript`)