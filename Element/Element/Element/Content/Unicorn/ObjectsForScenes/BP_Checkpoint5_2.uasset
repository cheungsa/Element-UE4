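; BP_Checkpoint5_2 is a checkpoint actor that shows billboard text and removes itself once all its assigned enemies are gone.
; On BeginPlay it copies its Text into the Widget_BillboardText widget held by the CheckPointText component.
; Each Tick it polls the Enemies array and destroys the actor when no entry is still valid, which also applies to an empty array.
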(event `self.ReceiveBeginPlay`
  (bind _aswidget_billboard_text (cast `/Game/Unicorn/ObjectsForScenes/Widget_BillboardText` (`WidgetComponent.GetUserWidgetObject` (`self.CheckPointText`))))
  (set `/Game/Unicorn/ObjectsForScenes/Widget_BillboardText.Text` (`self.text`) _aswidget_billboard_text))

(event `self.ReceiveActorBeginOverlap`
  (params (OtherActor :type "Actor Object Reference")))

(event `self.ReceiveTick`
  (params (DeltaSeconds :type "Float (single-precision)"))
  (set `self.ShouldDie` true)
  (for _array_element (`self.Enemies`)
    (if (`KismetSystemLibrary.IsValid` _array_element)
      (set `self.ShouldDie` false)
      (break)))
  (if (`self.ShouldDie`)
    (`self.K2_DestroyActor`)))

(fn `UserConstructionScript`)