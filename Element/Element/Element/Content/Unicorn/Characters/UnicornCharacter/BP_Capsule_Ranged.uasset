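; Ranged capsule character that attacks by shooting ice spike projectiles at its current target.
; The DoRangedAttack event calls ShootIceSpike, which spawns BP_IceSpike at the SpellLauncher and passes along the character's team.
; The spike is rotated toward the capsule controller's aim location on the target actor.
; Each shot then starts a one-shot timer lasting RangedAttackTime.
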(event `self.DoRangedAttack`
  (`self.ShootIceSpike`))

(fn `ShootIceSpike`
  (bind _returnvalue (`self.GetCapsuleController`))
  (bind _returnvalue_2 (`SceneComponent.K2_GetComponentLocation` (`self.SpellLauncher`)))
  (`|SpawnActorFromClass` "/Game/Unicorn/Spells/BP_IceSpike.BP_IceSpike_C" (`KismetMathLibrary.MakeTransform` _returnvalue_2 (`KismetMathLibrary.FindLookAtRotation` _returnvalue_2 (`UnicornAIController.GetAimLocationOnActor` _returnvalue (`UnicornAIController.GetTargetActor` _returnvalue)))) "Undefined" "OverrideRootScale" null 50.0 (1000.0 0.0 0.0) 3.0 (1.0 4.0 1.0) false 50.0 (0.0 0.0 0.0) 25.0 false 5.0 (`self.Team`) "TE_PlayerEnemy" null)
  (`KismetSystemLibrary.K2_SetTimerDelegate` (`|CreateDelegate` :!event `OnRangedAttackFinished`) (`self.RangedAttackTime`))
  (return))

(fn `UserConstructionScript`
  (`parent.UserConstructionScript`))