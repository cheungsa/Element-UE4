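; BP_Capsule_PortalMage is a capsule AI character with a randomized left, right or double melee attack and a ranged ice spike.
; Per-hand attack states, checked each Tick, drive timelines that extend hitboxes and reverse them on a hit or full extension.
; Hitbox overlaps damage actors on other teams, skipping those already hit.
; The spike spawns at the left eye toward the controller's target, passing team info.
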(event `self.ReceiveBeginPlay`
  (`parent.ReceiveBeginPlay`))

(event `self.HitboxRight.OnComponentBeginOverlap`
  (params (OverlappedComponent :type "PrimitiveComponent Object Reference") (OtherActor :type "Actor Object Reference") (OtherComp :type "PrimitiveComponent Object Reference") (OtherBodyIndex :type Integer) (bFromSweep :type Boolean) (SweepResult :type "HitResult Structure (by ref)"))
  (if (`|EnumEquality` (`self.AttackStateRight`) "NewEnumerator0")
    (`self.HitActor` OtherActor "NewEnumerator1")))

(event `self.HitboxLeft.OnComponentBeginOverlap`
  (params (OverlappedComponent :type "PrimitiveComponent Object Reference") (OtherActor :type "Actor Object Reference") (OtherComp :type "PrimitiveComponent Object Reference") (OtherBodyIndex :type Integer) (bFromSweep :type Boolean) (SweepResult :type "HitResult Structure (by ref)"))
  (if (`|EnumEquality` (`self.AttackStateLeft`) "NewEnumerator0")
    (`self.HitActor` OtherActor)))

(event `OnMeleeAttackFinishedLeft`
  (if (`|EnumEquality` (`self.AttackStateRight`) "NewEnumerator2")
    (`self.OnMeleeAttackFinished`)))

(event `self.ReceiveTick`
  (params (DeltaSeconds :type "Float (single-precision)"))
  (`parent.ReceiveTick` DeltaSeconds)
  (if (not (`self.bDead`))
    (`|ExecutionSequence`
      (:`then_0`
        (switch `/Game/Unicorn/Core/Engine/EAttackState` (`self.AttackStateLeft`)
          (:`NewEnumerator0`
            (bind (_direction _attacklefttime) (`Timeline|AttackLeftTimeline` :!label _label)
              (:`Update`
                (`SceneComponent.K2_SetRelativeLocation` (`self.HitboxLeft`) (`KismetMathLibrary.VLerp` (`self.HitboxPositionInactiveLeft`) (`self.HitboxPositionActiveLeft`) _attacklefttime) false false)
                (`SceneComponent.SetRelativeScale3D` (`self.HitboxLeft`) (`KismetMathLibrary.VLerp` (`self.HitboxLocalScaleInactive`) (`self.HitboxLocalScaleActive`) _attacklefttime)))
              (:`Finished`
                (switch `ETimelineDirection` _direction
                  (:`Forward`
                    (set `self.AttackStateLeft` "NewEnumerator1"))
                  (:`Backward`
                    (set `self.AttackStateLeft` "NewEnumerator2")
                    (`self.OnMeleeAttackFinishedLeft`))))))
          (:`NewEnumerator1`
            (goto _label :!via `Reverse`))))
      (:`then_1`
        (switch `/Game/Unicorn/Core/Engine/EAttackState` (`self.AttackStateRight`)
          (:`NewEnumerator0`
            (bind (_direction_2 _attacklefttime_2) (`Timeline|AttackRightTimeline` :!label _label_2)
              (:`Update`
                (`SceneComponent.K2_SetRelativeLocation` (`self.HitboxRight`) (`KismetMathLibrary.VLerp` (`self.HitboxPositionInactiveRight`) (`self.HitboxPositionActiveRight`) _attacklefttime_2) false false)
                (`SceneComponent.SetRelativeScale3D` (`self.HitboxRight`) (`KismetMathLibrary.VLerp` (`self.HitboxLocalScaleInactive`) (`self.HitboxLocalScaleActive`) _attacklefttime_2)))
              (:`Finished`
                (switch `ETimelineDirection` _direction_2
                  (:`Forward`
                    (set `self.AttackStateRight` "NewEnumerator1"))
                  (:`Backward`
                    (set `self.AttackStateRight` "NewEnumerator2")
                    (`self.OnMeleeAttackFinishedRight`))))))
          (:`NewEnumerator1`
            (goto _label_2 :!via `Reverse`)))))))

(event `OnMeleeAttackFinishedRight`
  (if (`|EnumEquality` (`self.AttackStateLeft`) "NewEnumerator2")
    (`self.OnMeleeAttackFinished`)))

(event `self.DoMeleeAttack`
  (`self.DoRandomMeleeAttack`))

(event `self.DoRangedAttack`
  (`self.ShootIceSpike`))

(fn `DoRandomMeleeAttack`
  (switch `int` (`KismetMathLibrary.RandomIntegerInRange` 0 2)
    (:`Default`
      (`self.MeleeAttack` "NewEnumerator0" :!label _label))
    (:`0`
      (`self.MeleeAttack` "NewEnumerator2"))
    (:`1`
      (`self.MeleeAttack` "NewEnumerator1"))
    (:`2`
      (goto _label)))
  (return))

(fn `HitActor`
  (params (HitActor :type "Actor Object Reference") (Hand :type "/Game/Unicorn/Core/Engine/EHand Enum" :default "NewEnumerator0"))
  (if (`TeamComponent.IsSameTeam` (`self.TeamComponent`) HitActor)
    _
    (elif (not (`KismetArrayLibrary.Array_Contains` (`self.HitActors`) (`local.HitActor`)))
      (`KismetArrayLibrary.Array_Add` (`self.HitActors`) (`local.HitActor`))
      (message `HealthInterface.LoseHealth` (`local.HitActor`) (`self.MeleeDamage`))
      (switch `/Game/Unicorn/Core/Engine/EHand` (`local.Hand`)
        (:`NewEnumerator0`
          (set `self.AttackStateLeft` "NewEnumerator1"))
        (:`NewEnumerator1`
          (set `self.AttackStateRight` "NewEnumerator1")))
      (return))))

(fn `MeleeAttack`
  (params (AttackType :type "/Game/Unicorn/Core/Engine/EHand Enum" :default "NewEnumerator0"))
  (switch `/Game/Unicorn/Core/Engine/EHand` AttackType
    (:`NewEnumerator0`
      (set `self.AttackStateLeft` "NewEnumerator0"))
    (:`NewEnumerator1`
      (set `self.AttackStateRight` "NewEnumerator0"))
    (:`NewEnumerator2`
      (`self.MeleeAttack` "NewEnumerator0")
      (`self.MeleeAttack` "NewEnumerator1")
      (return)))
  (for _array_element (`PrimitiveComponent.GetOverlappingActors` (select `/Game/Unicorn/Core/Engine/EHand` (`local.AttackType`) :`NewEnumerator0` (`self.HitboxLeft`) :`NewEnumerator1` (`self.HitboxRight`) :!type "PrimitiveComponent Object Reference") null)
    (`self.HitActor` _array_element))
  (return))

(fn `ShootIceSpike`
  (bind _returnvalue (`self.GetCapsuleController`))
  (bind _teamcomponent (`self.TeamComponent`))
  (bind _returnvalue_2 (`SceneComponent.K2_GetComponentLocation` (`self.LeftEye`)))
  (`|SpawnActorFromClass` "/Game/Unicorn/Spells/BP_IceSpike.BP_IceSpike_C" (`KismetMathLibrary.MakeTransform` _returnvalue_2 (`KismetMathLibrary.FindLookAtRotation` _returnvalue_2 (`UnicornAIController.GetAimLocationOnActor` _returnvalue (`UnicornAIController.GetTargetActor` _returnvalue)))) "Undefined" "OverrideRootScale" null 50.0 (1000.0 0.0 0.0) 3.0 (1.0 4.0 1.0) false 50.0 (0.0 0.0 0.0) 25.0 null false 5.0 (`TeamComponent.Team` _teamcomponent) (`TeamComponent.EnemyTeam` _teamcomponent) null)
  (`KismetSystemLibrary.K2_SetTimerDelegate` (`|CreateDelegate` :!event `OnRangedAttackFinished`) (`self.RangedAttackTime`))
  (return))

(fn `UserConstructionScript`
  (set `TeamComponent.Team` (`self.Team`) (`self.TeamComponent`))
  (bind _returnvalue (`KismetMaterialLibrary.CreateDynamicMaterialInstance` "/Game/Unicorn/Characters/UnicornCharacter/M_CapsuleMaterial.M_CapsuleMaterial"))
  (bind _output_get (set `self.BodyMat` _returnvalue))
  (`MaterialInstanceDynamic.SetVectorParameterValue` _output_get (`UnicornMaterialParameters.Color`) (`self.BodyColor`))
  (`PrimitiveComponent.SetMaterial` (`self.Sphere`) 0 (`self.BodyMat`))
  (`SceneComponent.SetRelativeScale3D` (`self.HitboxRight`) (`self.HitboxLocalScaleInactive`))
  (`SceneComponent.SetRelativeScale3D` (`self.HitboxLeft`) (`self.HitboxLocalScaleInactive`))
  (`SceneComponent.K2_SetRelativeLocation` (`self.HitboxRight`) (`self.HitboxPositionInactiveRight`) false false)
  (`SceneComponent.K2_SetRelativeLocation` (`self.HitboxLeft`) (`self.HitboxPositionInactiveLeft`) false false))