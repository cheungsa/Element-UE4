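; BP_CapsuleCharacter_Passive is a capsule character Blueprint whose death changes the text on four signs.
; Its OnDeath event writes a separate text variable to the text render of each referenced sign, then calls the parent death logic.
; BeginPlay, overlap and Tick are disabled stubs, and the construction script only calls the parent.
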(event `self.OnDeath`
  (`TextRenderComponent.K2_SetText` (`/Game/Unicorn/ObjectsForScenes/BP_SimpleSign.SignTextRender` (`self.Sign01`)) (`self.SignText01`))
  (`TextRenderComponent.K2_SetText` (`/Game/Unicorn/ObjectsForScenes/BP_SimpleSign.SignTextRender` (`self.Sign02`)) (`self.SignText02`))
  (`TextRenderComponent.K2_SetText` (`/Game/Unicorn/ObjectsForScenes/BP_SimpleSign.SignTextRender` (`self.Sign03`)) (`self.SignText03`))
  (`TextRenderComponent.K2_SetText` (`/Game/Unicorn/ObjectsForScenes/BP_SimpleSign.SignTextRender` (`self.Sign04`)) (`self.SignText04`))
  (`parent.OnDeath`))

(fn `UserConstructionScript`
  (`parent.UserConstructionScript`))