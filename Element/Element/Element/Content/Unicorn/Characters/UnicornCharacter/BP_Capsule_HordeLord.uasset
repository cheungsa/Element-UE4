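; BP_Capsule_HordeLord is a capsule character whose ranged attack summons portals toward its target.
; DoRangedAttack uses a randomized countdown so only every few attack calls fire, starting a RangedAttackTime timer either way.
; Despite its name, ShootIceSpike spawns a BT_Portal slightly ahead of the spell launcher, toward the target's aim location, with a small random spawn amount.
; The original BP_IceSpike projectile spawn remains in that function but is disconnected.
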(event `self.DoRangedAttack`
  (bind _spawndelay (`self.SpawnDelay`))
  (if (== 0 _spawndelay)
    (`self.ShootIceSpike`)
    (set `self.SpawnDelay` (`KismetMathLibrary.RandomIntegerInRange` 3 5))
    (else
      (bind _result (`/Engine/EditorBlueprintResources/StandardMacros.DecrementInt` _spawndelay)
        (:`  `
          (set `self.SpawnDelay` _result)
          (`KismetSystemLibrary.K2_SetTimerDelegate` (`|CreateDelegate` :!event `OnRangedAttackFinished`) (`self.RangedAttackTime`)))))))

(fn `ShootIceSpike`
  (bind _returnvalue (`self.GetCapsuleController`))
  (bind _returnvalue_2 (`SceneComponent.K2_GetComponentLocation` (`self.SpellLauncher`)))
  (bind _returnvalue_3 (`|SpawnActorFromClass` "/Game/Unicorn/Characters/UnicornCharacter/BT_Portal.BT_Portal_C" (`KismetMathLibrary.Conv_VectorToTransform` (+ _returnvalue_2 (* (`KismetMathLibrary.Conv_RotatorToVector` (`KismetMathLibrary.FindLookAtRotation` _returnvalue_2 (`UnicornAIController.GetAimLocationOnActor` _returnvalue (`UnicornAIController.GetTargetActor` _returnvalue)))) 200))) "AlwaysSpawn" "OverrideRootScale" null null))
  (set `/Game/Unicorn/Characters/UnicornCharacter/BT_Portal.m_SpawnAmount` (`KismetMathLibrary.RandomIntegerInRange` 2 4) _returnvalue_3)
  (`KismetSystemLibrary.K2_SetTimerDelegate` (`|CreateDelegate` :!event `OnRangedAttackFinished`) (`self.RangedAttackTime`))
  (return))

(fn `UserConstructionScript`
  (`parent.UserConstructionScript`))