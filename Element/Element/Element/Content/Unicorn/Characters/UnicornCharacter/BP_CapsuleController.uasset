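; AI controller for BP_CapsuleCharacter that maintains target and perception state.
; UpdateVision uses range and line-of-sight checks to acquire the player as target and write visibility to the Blackboard, starting a lost-target timer when sight fails.
; Stun component notifications set the stunned state.
; A target teleport while visible raises a timed recently-teleported flag, whose timer is cleared whenever visibility is set true.
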(event `self.ReceiveBeginPlay`
  (bind _asbp_capsule_character (cast `/Game/Unicorn/Characters/UnicornCharacter/BP_CapsuleCharacter` (`self.K2_GetPawn`)))
  (bind _bp_stuncomponent (`/Game/Unicorn/Characters/UnicornCharacter/BP_CapsuleCharacter.BP_StunComponent` _asbp_capsule_character))
  (add `/Game/Unicorn/Core/Engine/BP_StunComponent.NotifyStunBegin` _bp_stuncomponent (`|CreateDelegate` :!event `OnStunBegin`))
  (add `/Game/Unicorn/Core/Engine/BP_StunComponent.NotifyStunEnd` _bp_stuncomponent (`|CreateDelegate` :!event `OnStunEnd`)))

(event `OnStunBegin`
  (`self.SetStunned` true))

(event `OnStunEnd`
  (`self.SetStunned` false))

(event `self.OnTargetTeleported`
  ;[1 1 1] Update target teleported value
  (if (`self.GetCanSeeTarget`)
    (`KismetSystemLibrary.K2_ClearAndInvalidateTimerHandle` (`self.TargetRecentlyTeleportedTimer`))
    (`self.SetTargetRecentlyTeleported` true)
    (bind _returnvalue (`KismetSystemLibrary.K2_SetTimerDelegate` (delegate `TargetRecentlyTeleportedTimerExpired`) (`self.TargetRecentlyTeleportedTime`)))
    (set `self.TargetRecentlyTeleportedTimer` _returnvalue)))

(event `TargetRecentlyTeleportedTimerExpired`
  ;[1 1 1] Update target teleported value
  (`self.SetTargetRecentlyTeleported` false))

(event `LostTargetTimerExpired`
  (`self.SetTargetActor` null))

(fn `GetCanSeeTarget`
  (returns (ReturnValue :type Boolean))
  (locals (CanSeeTargetName :type Name :default "bCanSeeTarget"))
  (bind _blackboard (`self.Blackboard`))
  (`/Engine/EditorBlueprintResources/StandardMacros.IsValid` _blackboard
    (:`Is Valid`
      (return (`BlackboardComponent.GetValueAsBool` _blackboard (`local.CanSeeTargetName`))))))

(fn `SetCanSeeTarget`
  (params (bCanSeeTarget :type Boolean))
  (locals (CanSeeTargetName :type Name :default "bCanSeeTarget"))
  (bind _blackboard (`self.Blackboard`))
  (`/Engine/EditorBlueprintResources/StandardMacros.IsValid` _blackboard
    (:`Is Valid`
      (`BlackboardComponent.SetValueAsBool` _blackboard (`local.CanSeeTargetName`) (`local.bCanSeeTarget`))
      (if (`local.bCanSeeTarget`)
        (`KismetSystemLibrary.K2_ClearAndInvalidateTimerHandle` (`self.TargetRecentlyTeleportedTimer`))
        (else
          (`KismetSystemLibrary.K2_SetTimerDelegate` (`|CreateDelegate` :!event `LostTargetTimerExpired`) (`self.LostTargetTime`))))
      (return))))

(fn `UpdateVision`
  (`/Engine/EditorBlueprintResources/StandardMacros.IsValid` (`self.GetTargetActor`)
    (:`Is Valid`
      (if (<= (`KismetMathLibrary.VSize` (- (`self.K2_GetActorLocation` (`self.GetTargetActor`)) (`self.K2_GetActorLocation` (`self.K2_GetPawn`)))) (`self.LineOfSightRange`))
        (if (`self.LineOfSightTo` (`GameplayStatics.GetPlayerPawn` 0))
          (`self.SetCanSeeTarget` true)
          (else
            (`self.SetCanSeeTarget` false :!label _label)))
        (else
          (goto _label)))
      (return))
    (:`Is Not Valid`
      (`/Engine/EditorBlueprintResources/StandardMacros.IsValid` (`GameplayStatics.GetPlayerPawn` 0)
        (:`Is Valid`
          (if (<= (`KismetMathLibrary.VSize` (- (`self.K2_GetActorLocation` (`GameplayStatics.GetPlayerPawn` 0)) (`self.K2_GetActorLocation` (`self.K2_GetPawn`)))) (`self.LineOfSightRange`))
            (if (`self.LineOfSightTo` (`GameplayStatics.GetPlayerPawn` 0))
              (`self.SetTargetActor` (`GameplayStatics.GetPlayerPawn` 0))
              (`self.SetCanSeeTarget` true)
              (return))))))))

(fn `UserConstructionScript`)