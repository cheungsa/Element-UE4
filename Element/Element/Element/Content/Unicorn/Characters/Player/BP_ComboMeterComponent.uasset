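; Player combo meter component that tracks a clamped combo count and maps it to a four-level combo power.
; Each increment raises the count, re-evaluates power against low, medium and high thresholds, and restarts a reset timer.
; Timer expiry or an explicit reset returns count and power to their base values.
; The high-threshold check compares a constant zero instead of the current count.
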(event `ResetComboTimerExpired`
  (set `self.CurrComboCount` 0.0)
  (set `self.CurrComboPower` "NewEnumerator0"))

(fn `IncrementComboCount`
  ;[1 1 1] Update current count
  (set `self.CurrComboCount` (`KismetMathLibrary.FClamp` (+ (`self.CurrComboCount`) 1.0) 0.0 (`self.MaxComboCount`)))
  (`self.UpdateComboPower`)
  ;[1 1 1] Queue a reset of the combo timer
  (`KismetSystemLibrary.K2_ClearAndInvalidateTimerHandle` (`self.ComboResetTimer`))
  (bind _returnvalue (`KismetSystemLibrary.K2_SetTimerDelegate` (`|CreateDelegate` :!event `ResetComboTimerExpired`) (`self.ComboResetTime`)))
  (set `self.ComboResetTimer` _returnvalue)
  (return))

(fn `ResetComboCount`
  (`KismetSystemLibrary.K2_ClearAndInvalidateTimerHandle` (`self.ComboResetTimer`))
  (set `self.CurrComboCount` 0.0)
  (set `self.CurrComboPower` "NewEnumerator0")
  (return))

(fn `UpdateComboPower`
  (`|ExecutionSequence`
    (:`then_0`
      ;[1 1 1] Set the current combo power according to the thresholds
      (if (> 0.0 (`self.ComboThresholdHigh`))
        (set `self.CurrComboPower` "NewEnumerator3")
        (elif (> (`self.CurrComboCount`) (`self.ComboThresholdMed`))
          (set `self.CurrComboPower` "NewEnumerator2")
          (elif (> (`self.CurrComboCount`) (`self.ComboThresholdLow`))
            (set `self.CurrComboPower` "NewEnumerator1")
            (else
              (set `self.CurrComboPower` "NewEnumerator0"))))))
    (:`then_1`
      (return))))