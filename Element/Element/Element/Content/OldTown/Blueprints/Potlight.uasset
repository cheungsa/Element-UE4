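; Potlight is a recessed light fixture Blueprint that pairs a PotLight component with a SpotLight, with an on/off toggle and a single intensity control.
; The Construction Script creates a dynamic material instance on the fixture and drives both its emissive strength and the scaled spot light intensity from that control.
; Switching the toggle off zeroes both values, and the event graph holds no active logic.
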(fn `UserConstructionScript`
  (bind _intensity (`self.Intensity`))
  (bind _dmi (`self.DMI`))
  (bind _spotlight (`self.SpotLight`))
  (bind _returnvalue (`PrimitiveComponent.CreateDynamicMaterialInstance` (`self.PotLight`) 0 "/Game/OldTown/Materials/Spotlight.Spotlight"))
  (set `self.DMI` _returnvalue)
  (if (`self.Light Toggle`)
    (`MaterialInstanceDynamic.SetScalarParameterValue` _dmi "Emissive Strength" _intensity)
    (`LightComponent.SetIntensity` _spotlight (* _intensity 2500.0))
    (else
      (`MaterialInstanceDynamic.SetScalarParameterValue` _dmi "Emissive Strength" 0.0)
      (`LightComponent.SetIntensity` _spotlight 0.0))))