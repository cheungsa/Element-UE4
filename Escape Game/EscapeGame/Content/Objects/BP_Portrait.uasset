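; Portrait actor that stays hidden until the referenced piano puzzle is solved, then reveals a sprite and four text labels.
; The construction script fills the four text render components from Text variables.
; Every Tick polls the piano's PianoSolved flag and sets visibility of the sprite and labels to match, rather than reacting to an event.
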(event `self.ReceiveTick`
  (params (DeltaSeconds :type "Float (single-precision)"))
  (bind _textrender (`self.TextRender`))
  (bind _textrender1 (`self.TextRender1`))
  (bind _textrender3 (`self.TextRender3`))
  (bind _sprite_portrait (`self.Sprite_Portrait`))
  (bind _textrender2 (`self.TextRender2`))
  (if (`/Game/Blueprints/Widget_PianoPrompt.PianoSolved` (`self.RefPiano`))
    (`SceneComponent.SetVisibility` _sprite_portrait true false)
    (`SceneComponent.SetVisibility` _textrender true false)
    (`SceneComponent.SetVisibility` _textrender1 true false)
    (`SceneComponent.SetVisibility` _textrender2 true false)
    (`SceneComponent.SetVisibility` _textrender3 true false)
    (else
      (`SceneComponent.SetVisibility` _sprite_portrait false false)
      (`SceneComponent.SetVisibility` _textrender false false)
      (`SceneComponent.SetVisibility` _textrender1 false false)
      (`SceneComponent.SetVisibility` _textrender2 false false)
      (`SceneComponent.SetVisibility` _textrender3 false false))))

(fn `UserConstructionScript`
  (`TextRenderComponent.K2_SetText` (`self.TextRender`) (`self.Text1`))
  (`TextRenderComponent.K2_SetText` (`self.TextRender1`) (`self.Text2`))
  (`TextRenderComponent.K2_SetText` (`self.TextRender2`) (`self.Text3`))
  (`TextRenderComponent.K2_SetText` (`self.TextRender3`) (`self.Text4`)))