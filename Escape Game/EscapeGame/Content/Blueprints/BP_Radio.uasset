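; BP_Radio is an in-world radio that toggles a music track on and off.
; ToggleRadio uses a FlipFlop to spawn the sound at the actor's location, then stop the stored component.
; Each tick, a text prompt shows and turns toward the player's pawn when within range; otherwise it hides and the actor's input is disabled.
; The construction script sets the prompt from a Text variable.
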(event `/Game/Blueprints/BP_RadioInterface.ToggleRadio`
  (`/Engine/EditorBlueprintResources/StandardMacros.FlipFlop`
    (:`A`
      (bind _returnvalue (`GameplayStatics.SpawnSoundAtLocation` "/Game/Audio/Darkest_Child_-_Kevin_MacLeod__No_Copyright_Music_.Darkest_Child_-_Kevin_MacLeod__No_Copyright_Music_" (`self.K2_GetActorLocation`)))
      (set `self.SoundPlaying` _returnvalue))
    (:`B`
      (`AudioComponent.Stop` (`self.SoundPlaying`)))))

(event `self.ReceiveTick`
  (params (DeltaSeconds :type "Float (single-precision)"))
  (bind _textrender (`self.TextRender`))
  (if (< (`KismetMathLibrary.VSize` (- (`self.K2_GetActorLocation` (`Controller.K2_GetPawn` (`GameplayStatics.GetPlayerController` 0))) (`self.K2_GetActorLocation`))) 250.0)
    (`SceneComponent.SetVisibility` _textrender true false)
    (`SceneComponent.K2_SetWorldRotation` (`self.TextRender`) (`KismetMathLibrary.FindLookAtRotation` (`self.K2_GetActorLocation`) (`self.K2_GetActorLocation` (`Controller.K2_GetPawn` (`GameplayStatics.GetPlayerController` 0)))) false false)
    (else
      (`SceneComponent.SetVisibility` _textrender false false)
      (`self.DisableInput` (`GameplayStatics.GetPlayerController` 0)))))

(fn `UserConstructionScript`
  (`TextRenderComponent.K2_SetText` (`self.TextRender`) (`self.Text`)))