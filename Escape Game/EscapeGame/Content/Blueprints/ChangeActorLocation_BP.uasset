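; Blueprint that sets the location and rotation of the first player's controlled pawn at BeginPlay.
; A LoadedLevel flag chooses between the ActorLocation and ActorRotation variables and a PlayerStart's transform.
; Both branches require the controlled pawn itself to cast to PlayerStart, so a normal pawn stops the graph before any move.
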(event `BeginPlay`
  (if (`self.LoadedLevel`)
    (bind _asactor (cast `Actor` (`Controller.K2_GetPawn` (`GameplayStatics.GetPlayerController` 0))))
    (cast `PlayerStart` _asactor)
    (`Actor.K2_SetActorLocationAndRotation` (`Controller.K2_GetPawn` (`GameplayStatics.GetPlayerController` 0)) (`self.ActorLocation`) (`self.ActorRotation`) false false)
    (else
      (bind _asactor_2 (cast `Actor` (`Controller.K2_GetPawn` (`GameplayStatics.GetPlayerController` 0))))
      (bind _asplayer_start (cast `PlayerStart` _asactor_2))
      (`Actor.K2_SetActorLocationAndRotation` (`Controller.K2_GetPawn` (`GameplayStatics.GetPlayerController` 0)) (`Actor.K2_GetActorLocation` _asplayer_start) (`Actor.K2_GetActorRotation` _asplayer_start) false false))))